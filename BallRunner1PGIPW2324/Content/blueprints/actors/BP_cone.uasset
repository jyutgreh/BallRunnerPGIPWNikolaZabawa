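; BP_cone is a crystal pickup that flies into the player and vanishes when the player pawn overlaps its trigger.
; The CrystalTransform timeline pulls it toward the player's live position, shrinks it to zero and fades its light, then destroys it.
; Location and scale lerp from their current values each update, so the motion compounds.
; Any other overlapping actor only prints a Polish message about an enemy trying to steal the crystal.
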(event `self.trigger.OnComponentBeginOverlap`
  (params (OverlappedComponent :type "PrimitiveComponent Object Reference") (OtherActor :type "Actor Object Reference") (OtherComp :type "PrimitiveComponent Object Reference") (OtherBodyIndex :type Integer) (bFromSweep :type Boolean) (SweepResult :type "HitResult Structure (by ref)"))
  (if (== OtherActor (`GameplayStatics.GetPlayerPawn` 0))
    (bind (_direction _crystal_location _crystal_scale _crystal_light) (`Timeline|crystal transform`)
      (:`Update`
        (`self.K2_SetActorLocation` (`KismetMathLibrary.VLerp` (`self.K2_GetActorLocation`) (`self.K2_GetActorLocation` (`GameplayStatics.GetPlayerPawn` 0)) _crystal_location))
        (`self.SetActorScale3D` (`KismetMathLibrary.VLerp` (`self.GetActorScale3D`) (0.0 0.0 0.0) _crystal_scale))
        (`LightComponent.SetIntensity` (`self.crystallight`) (`KismetMathLibrary.Lerp` 2703.20166 0.0 _crystal_light)))
      (:`Finished`
        (`self.K2_DestroyActor`)))
    (else
      (`KismetSystemLibrary.PrintString` "Przeciwnik próbował ukrasc kryształ!"))))

(fn `UserConstructionScript`)