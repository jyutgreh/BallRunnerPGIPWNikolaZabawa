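; BP_Ball is a player-controlled rolling ball with an adjustable spring-arm camera view.
; ForwardBack and LeftRight axis inputs apply torque to the Sphere around Y and X, scaled by ForceMultiply as an acceleration change so mass is ignored.
; Change Camera View sets the spring arm's length, pitch and yaw from its parameters.
; A similarly named ChangeCameraView function is empty, with only disconnected nodes.
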(event `InputAxis|ForwardBack`
  (params (AxisValue :type "Float (single-precision)"))
  (`PrimitiveComponent.AddTorqueInRadians` (`self.Sphere`) (`KismetMathLibrary.MakeVector` 0.0 (* AxisValue (`self.force multiply`))) "None" true))

(event `InputAxis|LeftRight`
  (params (AxisValue :type "Float (single-precision)"))
  (`PrimitiveComponent.AddTorqueInRadians` (`self.Sphere`) (`KismetMathLibrary.MakeVector` (* AxisValue (`self.force multiply`))) "None" true))

(fn `Change Camera View`
  (params (`Camera Distance` :type "Float (double-precision)") (`Camera Rotation Y` :type "Float (double-precision)") (`Camera Rotation Z` :type "Float (double-precision)"))
  (bind _springarm (`self.SpringArm`))
  (set `SpringArmComponent.TargetArmLength` `Camera Distance` _springarm)
  (`SceneComponent.K2_SetRelativeRotation` _springarm (`KismetMathLibrary.MakeRotator` 0.0 `Camera Rotation Y` `Camera Rotation Z`) false false))

(fn `ChangeCameraView`)

(fn `UserConstructionScript`)